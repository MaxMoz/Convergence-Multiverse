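; DoctorFate is a playable character Blueprint with a sprint control and access to a character select menu.
; Holding Left Shift raises the movement component's max walk speed, and releasing it restores a slower walk.
; Tab creates a CharacterSelect widget, adds it to the viewport, disables the character's input and shows the mouse cursor.
; The construction script only calls its parent.
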(event `Key|Tab`
  (params (Key :type "Key Structure"))
  (bind _returnvalue (`GameplayStatics.GetPlayerController` 0))
  ;[1 1 1] Character Select Widget
  (:`Pressed`
    (bind _returnvalue_2 (`|CreateWidget` "/Game/Widgets/CharacterSelect.CharacterSelect_C"))
    (`UserWidget.AddToViewport` _returnvalue_2 0)
    (`self.DisableInput` _returnvalue)
    (set `PlayerController.bShowMouseCursor` true _returnvalue)))

(event `Key|LeftShift`
  (params (Key :type "Key Structure"))
  (bind _charactermovement (`self.CharacterMovement`))
  ;[1 1 1] Set Movement speed
  (:`Pressed`
    (set `CharacterMovementComponent.MaxWalkSpeed` 600.0 _charactermovement))
  (:`Released`
    (set `CharacterMovementComponent.MaxWalkSpeed` 150.0 _charactermovement)))

(fn `UserConstructionScript`
  (`parent.UserConstructionScript`))