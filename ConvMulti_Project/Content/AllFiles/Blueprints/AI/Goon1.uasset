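; Goon1 is an AI enemy that either roams the level or chases and punches the player.
; On BeginPlay it branches once on AIState to start the Roam or ChasePlayer loop.
; Roam moves to random navigable points near its current location, pausing between moves.
; ChasePlayer moves to the player, plays a punch montage, waits and repeats; both loops continue only when a move succeeds.
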(event `self.ReceiveBeginPlay`
  (switch `/Game/AllFiles/Blueprints/AI/AIType` (`self.AIState`)
    (:`NewEnumerator1`
      (`self.Roam`))
    (:`NewEnumerator2`
      (`self.ChasePlayer`))))

(event `Roam`
  (`|AIMoveTo` self (`NavigationSystemV1.K2_GetRandomLocationInNavigableRadius` (`self.K2_GetActorLocation`) 1500.0 null null) null 100.0
    (:`OnSuccess`
      (`KismetSystemLibrary.Delay` 2.0)
      (`self.Roam`))))

(event `ChasePlayer`
  (`|AIMoveTo` self (0.0 0.0 0.0) (`GameplayStatics.GetPlayerCharacter` 0) 100.0
    (:`OnSuccess`
      (`self.PlayAnimMontage` "/Game/AIVillains/Goon1/Anims/GoonPunching.GoonPunching")
      (`KismetSystemLibrary.Delay` 1.0)
      (`self.ChasePLayer`))))

(fn `UserConstructionScript`)