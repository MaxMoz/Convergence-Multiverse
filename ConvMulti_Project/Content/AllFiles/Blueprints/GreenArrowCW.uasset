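; GreenArrowCW is a character Blueprint that adds hold-to-sprint and a close-view camera.
; Left Shift switches CharacterMovement's max walk speed between walk and run values and sets the IsRunning flag.
; Holding the right mouse button moves FollowCamera to a fixed relative offset with MoveComponentTo, and releasing it moves the camera to the node's default target location.
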(event `Key|LeftShift`
  (params (Key :type "Key Structure"))
  (bind _charactermovement (`self.CharacterMovement`))
  ;[1 1 1] Set Movement speed
  (:`Pressed`
    (set `CharacterMovementComponent.MaxWalkSpeed` 450.0 _charactermovement))
  (:`Released`
    (set `CharacterMovementComponent.MaxWalkSpeed` 150.0 _charactermovement)))

(event `Key|LeftShift`
  (params (Key :type "Key Structure"))
  ;[1 1 1] Set Running Variable
  (:`Pressed`
    (set `self.Is_Running` true))
  (:`Released`
    (set `self.Is_Running` false)))

(event `Key|RightMouseButton`
  (params (Key :type "Key Structure"))
  (bind _followcamera (`self.FollowCamera`))
  ;[1 1 1] Close View Camera
  (:`Pressed`
    (`KismetSystemLibrary.MoveComponentTo` _followcamera (226.759216 43.081039 44.587212)))
  (:`Released`
    (`KismetSystemLibrary.MoveComponentTo` _followcamera)))

(fn `UserConstructionScript`
  (`parent.UserConstructionScript`))