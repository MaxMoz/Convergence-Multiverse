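; RF52 is a Flash-style speedster character Blueprint with keyboard-driven powers and a health bar widget created on BeginPlay.
; Left Shift toggles held super speed and Left Ctrl a moderate run; during super speed, Tick shakes the camera and shifts FollowCamera backward.
; Holding Q phases through WorldStatic by changing capsule collision, with a camera shake on press.
; E toggles slow motion through the actor's own CustomTimeDilation.
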(event `Key|E`
  (params (Key :type "Key Structure"))
  ;[1 1 1] Slo Mo Camera
  (:`Pressed`
    (`/Engine/EditorBlueprintResources/StandardMacros.FlipFlop`
      (:`A`
        (set `self.CustomTimeDilation` 0.05))
      (:`B`
        (set `self.CustomTimeDilation` 1.0)))))

(event `Key|LeftControl`
  (params (Key :type "Key Structure"))
  (bind _charactermovement (`self.CharacterMovement`))
  ;[1 1 1] Set Movement speed
  (:`Pressed`
    (set `CharacterMovementComponent.MaxWalkSpeed` 450.0 _charactermovement))
  (:`Released`
    (set `CharacterMovementComponent.MaxWalkSpeed` 150.0 _charactermovement)))

(event `Key|Q`
  (params (Key :type "Key Structure"))
  (bind _capsulecomponent (`self.CapsuleComponent`))
  ;[1 1 1] Phazing
  (:`Pressed`
    (set `self.Is_Phasing` true)
    (`PrimitiveComponent.SetCollisionResponseToChannel` _capsulecomponent "ECC_WorldStatic" "ECR_Ignore")
    (`GameplayStatics.PlayWorldCameraShake` "/Game/Characters/FlashCW/FlashHUD/PhasingShake.PhasingShake_C" (`self.K2_GetActorLocation`) 0.0 300.0 1.0 true))
  (:`Released`
    (set `self.Is_Phasing` false)
    (`PrimitiveComponent.SetCollisionResponseToAllChannels` _capsulecomponent "ECR_Block")))

(event `self.ReceiveTick`
  (params (DeltaSeconds :type "Float (single-precision)"))
  (bind _followcamera (`self.FollowCamera`))
  ;[1 1 1] Running Effects
  (`|ExecutionSequence`
    (:`then_0`
      (if (`self.Is_SuperSpeed`)
        (`|ExecutionSequence`
          (:`then_0`
            (`GameplayStatics.PlayWorldCameraShake` "/Game/Characters/FlashCW/FlashHUD/PhasingShake.PhasingShake_C" (`self.K2_GetActorLocation`) 0.0 500.0))
          (:`then_1`
            (`KismetSystemLibrary.MoveComponentTo` _followcamera (-22.675095 0.0 0.0))))
        (else
          (`KismetSystemLibrary.MoveComponentTo` _followcamera (28.841003 0.0 0.0) (struct) false false 0.1))))))

(event `self.ReceiveBeginPlay`
  ;[1 1 1] Health Bar
  (bind _returnvalue (`|CreateWidget` "/Game/Characters/FlashCW/FlashHUD/FlashHealthBar.FlashHealthBar_C"))
  (`UserWidget.AddToViewport` _returnvalue 0))

(event `Key|LeftShift`
  (params (Key :type "Key Structure"))
  (bind _charactermovement (`self.CharacterMovement`))
  ;[1 1 1] Set SuperSpeed
  (:`Pressed`
    (set `self.Is_SuperSpeed` true)
    (set `CharacterMovementComponent.MaxWalkSpeed` 3000.0 _charactermovement))
  (:`Released`
    (set `self.Is_SuperSpeed` false)
    (set `CharacterMovementComponent.MaxWalkSpeed` 150.0 _charactermovement)))

(fn `UserConstructionScript`
  (`parent.UserConstructionScript`))